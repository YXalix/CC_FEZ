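; Player hero Blueprint for a platformer where the camera turns in quarter steps and cube collision follows the view.
; Turn inputs call MovetoPoint, rotate the spring arm by timeline, update FaceKind, then swap every cube's collision X/Y scale.
; Jumping at location type 3 stretches nearby cubes' collision along X; ChangeCollisionDirection resets tag "2" cubes of that type to unit scale.
; The GameOver visibility check is unconnected.
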(event `self.ReceiveTick`
  (params (DeltaSeconds :type "Float (single-precision)")))

(event `self.MyJump`
  (bind _returnvalue (`self.K2_GetActorLocation`))
  (`self.Jump`)
  (bind _returnvalue_2 (`self.GetLevelLocationInfo` _returnvalue))
  (if (== _returnvalue_2 3)
    (bind _returnvalue_3 (`self.GetCubesByHeroLocation` _returnvalue))
    (for _array_element _returnvalue_3
      (bind _asbp_cube (cast `/Game/Meshes/BP_Cube` _array_element))
      (`KismetSystemLibrary.PrintString` (`KismetStringLibrary.Conv_VectorToString` (`self.K2_GetActorLocation` _asbp_cube)) true true (struct :`G` 0.66 :`B` 1.0 :`A` 1.0) 20.0)
      (`SceneComponent.SetWorldScale3D` (`/Game/Meshes/BP_Cube.Collision` _asbp_cube) (64.0 1.0 1.0)))))

(event `self.MyStopJump`
  (`self.StopJumping`))

(event `InputAction|TurnLeft`
  (params (Key :type "Key Structure"))
  ;[1 1 1] TurnLeft
  (:`Pressed`
    (`self.UpdateInfo`)
    (`self.MovetoPoint`)
    (bind (_direction _z_r) (`Timeline|Timeline_0` :!via `PlayFromStart`)
      (:`Update`
        (`SceneComponent.K2_SetWorldRotation` (`self.SpringArm`) (`KismetMathLibrary.MakeRotator` 0.0 0.0 (+ (* (`self.FaceKind`) 90.0) _z_r)) false false))
      (:`Finished`
        (`self.FaceKindAdd`)
        (bind _outactors (`GameplayStatics.GetAllActorsOfClass` "/Game/Meshes/BP_Cube.BP_Cube_C"))
        (for _array_element _outactors
          (bind _collision (`/Game/Meshes/BP_Cube.Collision` _array_element))
          (bind (_returnvalue_x _returnvalue_y _returnvalue_z) (`KismetMathLibrary.BreakVector` (`SceneComponent.K2_GetComponentScale` _collision)))
          (`SceneComponent.SetWorldScale3D` _collision (`KismetMathLibrary.MakeVector` _returnvalue_y _returnvalue_x _returnvalue_z)))))))

(event `InputAction|TurnRight`
  (params (Key :type "Key Structure"))
  ;[1 1 1] TurnRight
  (:`Pressed`
    (`self.UpdateInfo`)
    (`self.MovetoPoint`)
    (bind (_direction _z_r) (`Timeline|Timeline_1` :!via `PlayFromStart`)
      (:`Update`
        (`SceneComponent.K2_SetWorldRotation` (`self.SpringArm`) (`KismetMathLibrary.MakeRotator` 0.0 0.0 (+ (* (`self.FaceKind`) 90.0) _z_r)) false false))
      (:`Finished`
        (`self.FaceKindSub`)
        (bind _outactors (`GameplayStatics.GetAllActorsOfClass` "/Game/Meshes/BP_Cube.BP_Cube_C"))
        (for _array_element _outactors
          (bind _collision (`/Game/Meshes/BP_Cube.Collision` _array_element))
          (bind (_returnvalue_x _returnvalue_y _returnvalue_z) (`KismetMathLibrary.BreakVector` (`SceneComponent.K2_GetComponentScale` _collision)))
          (`SceneComponent.SetWorldScale3D` _collision (`KismetMathLibrary.MakeVector` _returnvalue_y _returnvalue_x _returnvalue_z)))))))

(event `InputAction|ChangeCollisionDirection`
  (params (Key :type "Key Structure"))
  (:`Pressed`
    (bind _outactors (`GameplayStatics.GetAllActorsOfClassWithTag` "/Game/Meshes/BP_Cube.BP_Cube_C" "2"))
    (for _array_element _outactors
      (bind _returnvalue (`self.GetLevelLocationInfo` (`self.K2_GetActorLocation` _array_element)))
      (if (== _returnvalue 3)
        (`SceneComponent.SetWorldScale3D` (`/Game/Meshes/BP_Cube.Collision` _array_element) (1.0 1.0 1.0))))))

(fn `UserConstructionScript`)